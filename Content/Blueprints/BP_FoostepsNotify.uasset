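; PaperZD animation notify that plays Hope's footstep sounds according to the surface underfoot.
; On receipt, it traces down from the owning actor along its up vector on the Visibility channel and reads the hit's surface type.
; Grass, stone or wood sounds play at the sequence render component's location, with grass as the fallback for other surfaces.
; A trace miss plays nothing, and an invalid owning instance prints a debug message.
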(event `self.OnReceiveNotify`
  (params (OwningInstance :type "PaperZDAnimInstance Object Reference"))
  (bind _returnvalue (`SceneComponent.K2_GetComponentLocation` (`self.SequenceRenderComponent`)))
  (`/Engine/EditorBlueprintResources/StandardMacros.IsValid` OwningInstance
    (:`Is Valid`
      (bind _output_get (set `self.NewVar` (`PaperZDAnimInstance.GetOwningActor` OwningInstance)))
      (bind _returnvalue_2 (`Actor.K2_GetActorLocation` _output_get))
      (bind (_outhit _returnvalue_3) (`KismetSystemLibrary.LineTraceSingle` _returnvalue_2 (+ _returnvalue_2 (* (`Actor.GetActorUpVector` _output_get) -200.0)) "TraceTypeQuery1"))
      (if _returnvalue_3
        (switch `EPhysicalSurface` (`GameplayStatics.GetSurfaceType` _outhit)
          (:`SurfaceType_Default`
            (`GameplayStatics.PlaySoundAtLocation` "/Game/Assets/SD/SFXQ/Hope/Steps/SFX_HOPE_STEP_GRASS.SFX_HOPE_STEP_GRASS" _returnvalue (struct) 1.0 1.0 0.0 null null null null :!label _label))
          (:`SurfaceType1`
            (goto _label))
          (:`SurfaceType2`
            (`GameplayStatics.PlaySoundAtLocation` "/Game/Assets/SD/SFXQ/Hope/Steps/SFX_HOPE_STEP_STONE.SFX_HOPE_STEP_STONE" _returnvalue (struct) 1.0 1.0 0.0 null null null null))
          (:`SurfaceType3`
            (`GameplayStatics.PlaySoundAtLocation` "/Game/Assets/SD/SFXQ/Hope/Steps/SFX_HOPE_STEP_WOOD.SFX_HOPE_STEP_WOOD" _returnvalue (struct) 1.0 1.0 0.0 null null null null)))))
    (:`Is Not Valid`
      (`KismetSystemLibrary.PrintString` "Footstep Notify Iwning Instance Not Valid"))))