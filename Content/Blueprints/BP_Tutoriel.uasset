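; Tutorial trigger volume that makes an interaction text available to the player character, BP_Hope.
; BeginPlay caches the player as BP_Hope.
; Box overlap begin sets that character's interaction flag and copies in this actor's Txte, and overlap end clears only the flag.
; Overlaps check that the player exists, not which actor overlapped, and the interaction image assignment is disconnected.
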(event `self.ReceiveBeginPlay`
  (bind _asbp_hope (cast `/Game/Blueprints/Hope/BP_Hope` (`GameplayStatics.GetPlayerCharacter` 0)))
  (set `self.As BP Hope` _asbp_hope))

(event `self.Box.OnComponentBeginOverlap`
  (params (OverlappedComponent :type "PrimitiveComponent Object Reference") (OtherActor :type "Actor Object Reference") (OtherComp :type "PrimitiveComponent Object Reference") (OtherBodyIndex :type Integer) (bFromSweep :type Boolean) (SweepResult :type "HitResult Structure (by ref)"))
  (`/Engine/EditorBlueprintResources/StandardMacros.IsValid` (`GameplayStatics.GetPlayerCharacter` 0)
    (:`Is Valid`
      (set `/Game/Blueprints/Hope/BP_Hope.isInteractionPossible?` true (`self.As BP Hope`))
      (set `/Game/Blueprints/Hope/BP_Hope.TexteInteraction` (`self.Txte`) (`self.As BP Hope`)))))

(event `self.Box.OnComponentEndOverlap`
  (params (OverlappedComponent :type "PrimitiveComponent Object Reference") (OtherActor :type "Actor Object Reference") (OtherComp :type "PrimitiveComponent Object Reference") (OtherBodyIndex :type Integer))
  (`/Engine/EditorBlueprintResources/StandardMacros.IsValid` (`GameplayStatics.GetPlayerCharacter` 0)
    (:`Is Valid`
      (set `/Game/Blueprints/Hope/BP_Hope.isInteractionPossible?` false (`self.As BP Hope`)))))

(fn `UserConstructionScript`)