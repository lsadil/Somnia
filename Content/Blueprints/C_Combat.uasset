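; C_Combat is a combat Blueprint that provides hit detection, health reduction and death handling.
; HitCheck applies base damage to the first actor other than itself overlapping a given box collision, then returns true.
; ReceiveDamage subtracts incoming damage from Health and calls Death at zero or below, which removes the given actor through a very short life span.
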(fn `Death`
  (params (Actor :type "Actor Object Reference"))
  (`Actor.SetLifeSpan` Actor 0.01))

(fn `Hit + Check`
  (params (`Box Collision` :type "BoxComponent Object Reference"))
  (returns (Hit :type Boolean))
  (for _array_element (`PrimitiveComponent.GetOverlappingActors` `Box Collision` null)
    (if (!= _array_element self)
      (`GameplayStatics.ApplyDamage` _array_element (`self.Base Damage`))
      (return true))))

(fn `Receive Damage`
  (params (ReceivedDamage :type "Float (double-precision)") (Actor :type "Actor Object Reference"))
  (bind _output_get (set `self.Health` (- (`self.Health`) ReceivedDamage)))
  (if (<= _output_get 0.0)
    (`self.Death` Actor)))