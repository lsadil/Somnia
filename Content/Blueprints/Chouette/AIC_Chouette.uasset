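; AI controller for the Chouette enemy that runs its behavior tree on begin play.
; Perception updates store any detected BP_Hope actor in the blackboard's Player key, with no check on whether it is sensed or lost.
; The Dead event stops the brain logic, while the writes for attack and patrol cooldowns are present but never run.
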(event `Dead`
  (`BrainComponent.StopLogic` (`self.BrainComponent`) "Dead"))

(event `self.ReceiveBeginPlay`
  (`self.RunBehaviorTree` "/Game/Blueprints/Chouette/BT_Chouette.BT_Chouette")
  (cast `/Game/Blueprints/Chouette/BP_Chouette` (`self.K2_GetPawn`)))

(event `self.AIPerception.OnPerceptionUpdated`
  (params (UpdatedActors :type "Array of Actor Object Reference (by ref)"))
  (for _array_element UpdatedActors
    ;[1 1 1] TODO : Interface
    (bind _asbp_hope (cast `/Game/Blueprints/Hope/BP_Hope` _array_element))
    (`BlackboardComponent.SetValueAsObject` (`AIBlueprintHelperLibrary.GetBlackboard` null) "Player" _asbp_hope)))

(fn `UserConstructionScript`)