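; BP_Chouette is a sprite-based AI character that takes damage and tracks which side the player is on.
; On BeginPlay it copies Health and Damage into its Combat component and creates a dynamic sprite material.
; While not idle, Tick sets Direction from the player's X position.
; Damage notifies AIC_Chouette, passes through Combat, sets Hit and triggers a timeline-driven red material flash.
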(event `self.ReceiveBeginPlay`
  (bind _returnvalue (`PrimitiveComponent.CreateDynamicMaterialInstance` (`self.Sprite`) 0 null "None"))
  (set `self.Dynamic Sprite Mat` _returnvalue)
  (set `/Game/Blueprints/C_Combat.Health` (`self.Health`) (`self.Combat`))
  (set `/Game/Blueprints/C_Combat.Base Damage` (`self.Damage`) (`self.Combat`)))

(event `self.ReceiveTick`
  (params (DeltaSeconds :type "Float (single-precision)"))
  (if (not (`self.Idle`))
    (bind _direction (`self.FacePlayer`))
    (set `self.Direction` _direction)))

(event `self.ReceiveAnyDamage`
  (params (Damage :type "Float (single-precision)") (DamageType :type "DamageType Object Reference") (InstigatedBy :type "Controller Object Reference") (DamageCauser :type "Actor Object Reference"))
  (bind _asaic_chouette (cast `/Game/Blueprints/Chouette/AI/AIC_Chouette` (`self.GetController`)))
  (`/Game/Blueprints/Chouette/AI/AIC_Chouette.Hit` _asaic_chouette)
  (`/Game/Blueprints/C_Combat.Receive Damage` (`self.Combat`) Damage self)
  (`self.TriggerFlash` 1.0)
  (set `self.Hit` true))

(event `TriggerFlash`
  (params (Multiplier :type "Float (single-precision)" :default 1.0) (Color :type "LinearColor Structure" :default (struct :`R` 1.0 :`A` 1.0)) (`Play Rate` :type "Float (single-precision)" :default 5.0))
  (`MaterialInstanceDynamic.SetScalarParameterValue` (`self.Dynamic Sprite Mat`) "Flash Multiplier" Multiplier)
  (`MaterialInstanceDynamic.SetVectorParameterValue` (`self.Dynamic Sprite Mat`) "Flash Color" Color)
  (`TimelineComponent.SetPlayRate` (`self.Timeline`) `Play Rate`)
  (bind (_direction _alpha) (`Timeline|Timeline` :!via `PlayFromStart`)
    (:`Update`
      (`MaterialInstanceDynamic.SetScalarParameterValue` (`self.Dynamic Sprite Mat`) "Flash Multiplier" (`KismetMathLibrary.Lerp` 0.0 Multiplier _alpha)))))

(fn `FacePlayer`
  (returns (Direction :type "Float (double-precision)"))
  (bind _returnvalue_x (`KismetMathLibrary.BreakVector` (`self.K2_GetActorLocation`)))
  (bind _returnvalue_x_2 (`KismetMathLibrary.BreakVector` (`self.K2_GetActorLocation` (`GameplayStatics.GetPlayerPawn` 0))))
  (if (> _returnvalue_x_2 _returnvalue_x)
    (return 0.0)
    (else
      (return -180.0))))

(fn `UserConstructionScript`)