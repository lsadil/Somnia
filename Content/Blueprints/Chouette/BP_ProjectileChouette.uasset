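; BP_ProjectileChouette is a projectile, named for the owl (Chouette), that damages the player character BP_Hope.
; It caches Hope on BeginPlay, and when its Box overlaps her it applies fixed damage and destroys itself.
; Overlaps with other actors are ignored, and a tornado-spell collision branch through ACCollisionTornado is present but never runs.
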(event `self.ReceiveBeginPlay`
  (bind _asbp_hope (cast `/Game/Blueprints/Hope/BP_Hope` (`GameplayStatics.GetPlayerCharacter` 0)))
  (set `self.Hope` _asbp_hope))

(event `self.Box.OnComponentBeginOverlap`
  (params (OverlappedComponent :type "PrimitiveComponent Object Reference") (OtherActor :type "Actor Object Reference") (OtherComp :type "PrimitiveComponent Object Reference") (OtherBodyIndex :type Integer) (bFromSweep :type Boolean) (SweepResult :type "HitResult Structure (by ref)"))
  (if (== OtherActor (`self.Hope`))
    (`GameplayStatics.ApplyDamage` (`self.Hope`) 10.0)
    (`self.K2_DestroyActor`)))

(fn `UserConstructionScript`)