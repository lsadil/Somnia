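; BP_DialogueForced is a one-shot trigger that forces a dialogue to open when BP_Hope enters its sphere.
; On overlap, it picks the French or English data table from the language flag in GM_Base.
; It writes that table to BP_Hope, then, if the table is valid, adds a Dialogue_HUD widget to the viewport and destroys itself.
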(event `self.Sphere.OnComponentBeginOverlap`
  (params (OverlappedComponent :type "PrimitiveComponent Object Reference") (OtherActor :type "Actor Object Reference") (OtherComp :type "PrimitiveComponent Object Reference") (OtherBodyIndex :type Integer) (bFromSweep :type Boolean) (SweepResult :type "HitResult Structure (by ref)"))
  (bind _data_table_selected (`self.Data Table Selected`))
  (`|ExecutionSequence`
    (:`then_0`
      (bind _asgm_base (cast `/Game/Blueprints/GM_Base` (`GameplayStatics.GetGameMode`)))
      (if (`/Game/Blueprints/GM_Base.Français` _asgm_base)
        (set `self.Data Table Selected` (`self.Data Table Français`))
        (else
          (set `self.Data Table Selected` (`self.Data Table English`)))))
    (:`then_1`
      (bind _asbp_hope (cast `/Game/Blueprints/Hope/BP_Hope` OtherActor))
      (set `/Game/Blueprints/Hope/BP_Hope.Data Table Dialogue` _data_table_selected _asbp_hope)
      (`/Engine/EditorBlueprintResources/StandardMacros.IsValid` _data_table_selected
        (:`Is Valid`
          (bind _returnvalue (`|CreateWidget` "/Game/Blueprints/UI/Blueprints/Dialogue_HUD.Dialogue_HUD_C"))
          (`UserWidget.AddToViewport` _returnvalue 0)
          (`self.K2_DestroyActor`))))))

(fn `UserConstructionScript`)