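; Sprite-based enemy actor that takes damage and reacts to the tornado spell.
; On BeginPlay it copies its Health and Damage into the Combat component and creates a dynamic material for the sprite.
; While alive, damage goes to Combat and triggers a red flash, driven by a Timeline animating material parameters.
; Overlapping a BP_MagicSpell_Tornado hands the enemy to the ACCollisionTornado component.
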(event `self.ReceiveBeginPlay`
  (bind _combat (`self.Combat`))
  (set `/Game/Blueprints/C_Combat.Health` (`self.Health`) _combat)
  (set `/Game/Blueprints/C_Combat.Base Damage` (`self.Damage`) _combat)
  (bind _returnvalue (`PrimitiveComponent.CreateDynamicMaterialInstance` (`self.Sprite`) 0 null "None"))
  (set `self.Dynamic Sprite Mat` _returnvalue))

(event `self.ReceiveAnyDamage`
  (params (Damage :type "Float (single-precision)") (DamageType :type "DamageType Object Reference") (InstigatedBy :type "Controller Object Reference") (DamageCauser :type "Actor Object Reference"))
  (bind _combat (`self.Combat`))
  (if (not (`/Game/Blueprints/C_Combat.Dead` _combat))
    (`/Game/Blueprints/C_Combat.Receive Damage` _combat Damage self)
    (`self.TriggerFlash` 1.0 (struct :`R` 1.0 :`A` 1.0) 10.0)))

(event `TriggerFlash`
  (params (Multiplier :type "Float (single-precision)" :default 1.0) (Color :type "LinearColor Structure" :default (struct :`R` 1.0 :`A` 1.0)) (`Play Rate` :type "Float (single-precision)" :default 5.0))
  (`MaterialInstanceDynamic.SetScalarParameterValue` (`self.Dynamic Sprite Mat`) "Flash Multiplier" Multiplier)
  (`MaterialInstanceDynamic.SetVectorParameterValue` (`self.Dynamic Sprite Mat`) "Flash Color" Color)
  (`TimelineComponent.SetPlayRate` (`self.Timeline`) `Play Rate`)
  (bind (_direction _alpha) (`Timeline|Timeline` :!via `PlayFromStart`)
    (:`Update`
      (`MaterialInstanceDynamic.SetScalarParameterValue` (`self.Dynamic Sprite Mat`) "Flash Multiplier" (`KismetMathLibrary.Lerp` 0.0 Multiplier _alpha)))))

(event `self.ReceiveActorBeginOverlap`
  (params (OtherActor :type "Actor Object Reference"))
  (if (== (`GameplayStatics.GetObjectClass` OtherActor) "/Game/Blueprints/Runes/Runes_MagicSpells/BP_MagicSpell_Tornado.BP_MagicSpell_Tornado_C")
    (`/Game/Blueprints/Mechanics/AC_CollisionTornado.TornadoCollision` (`self.AC_CollisionTornado`) self)))

(event `self.ReceiveDestroyed`)

(fn `UserConstructionScript`)