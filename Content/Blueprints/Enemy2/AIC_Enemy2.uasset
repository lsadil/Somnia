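; AI controller for Enemy2 that runs its behavior tree and feeds the blackboard.
; On BeginPlay it starts BT_Enemy2 and copies the controlled pawn's Cooldown into the blackboard.
; When AI perception updates on a BP_Hope actor, it stores that actor as the Player key and sets CanSeePlayer on the pawn.
; That flag is only ever set true here, with no handling for losing sight.
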(event `self.ReceiveBeginPlay`
  (`self.RunBehaviorTree` "/Game/Blueprints/Enemy2/BT_Enemy2.BT_Enemy2")
  (bind _asbp_enemy_2 (cast `/Game/Blueprints/Enemy2/BP_Enemy2` (`self.K2_GetPawn`)))
  (`BlackboardComponent.SetValueAsFloat` (`AIBlueprintHelperLibrary.GetBlackboard` null) "Cooldown" (`/Game/Blueprints/Enemy2/BP_Enemy2.Cooldown` _asbp_enemy_2)))

(event `self.AIPerception.OnTargetPerceptionUpdated`
  (params (Actor :type "Actor Object Reference") (Stimulus :type "AIStimulus Structure"))
  ;[1 1 1] TODO : Interface
  (bind _asbp_hope (cast `/Game/Blueprints/Hope/BP_Hope` Actor))
  (bind _output_get (set `self.As BP Hope` _asbp_hope))
  (`BlackboardComponent.SetValueAsObject` (`AIBlueprintHelperLibrary.GetBlackboard` null) "Player" _output_get)
  (bind _asbp_enemy_2 (cast `/Game/Blueprints/Enemy2/BP_Enemy2` (`self.K2_GetPawn`)))
  (set `/Game/Blueprints/Enemy2/BP_Enemy2.Can See Player` true _asbp_enemy_2))

(fn `UserConstructionScript`)