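; Side-scrolling enemy character that patrols along the X axis, attacks the player and dies when health runs out.
; Forward and downward-diagonal line traces detect obstacles and ledges, triggering a pause and turnaround through a shared DoOnce.
; Box overlap runs a looping timer for the attack animation, while a separate Attack event traces forward to damage the player.
; Damage turns it toward the attacker, then applies knockback or plays death before destroying it.
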(event `self.ReceiveBeginPlay`
  (set `CharacterMovementComponent.MaxWalkSpeed` (`self.Max Walk Speed`) (`self.CharacterMovement`)))

(event `self.ReceiveTick`
  (params (DeltaSeconds :type "Float (single-precision)"))
  (`self.Rotation`)
  (`self.Movement`))

(event `Rotation`
  ;[1 1 1] Rotation
  (if (`self.IsDead`)
    _
    (elif (> (`self.Direction`) 0.0)
      (`self.K2_SetActorRotation` (struct))
      (else
        (`self.K2_SetActorRotation` (struct :`Yaw` 180.0))))))

(event `Movement`
  (bind _returnvalue (`self.K2_GetActorLocation`))
  (bind _returnvalue_2 (`self.K2_GetActorLocation`))
  ;[1 1 1] Movement
  (if (not (or (`self.IsDead`) (`self.Damaged`)))
    ;;[1 1 1] Commence dans la direction
    (`self.AddMovementInput` (1.0 0.0 0.0) (`self.Direction`))
    (`|ExecutionSequence`
      (:`then_0`
        ;;[1 1 1] Rotation obstacle
        (bind (_outhit _returnvalue_3) (`KismetSystemLibrary.LineTraceSingleForObjects` _returnvalue (+ _returnvalue (* (`self.GetActorForwardVector`) (150.0 0.0 0.0))) (`|MakeArray` "ObjectTypeQuery1" "ObjectTypeQuery2" "ObjectTypeQuery3" :!type "EObjectTypeQuery Enum") false (`|MakeArray` (`GameplayStatics.GetPlayerCharacter` 0) :!type "Actor Object Reference") "ForOneFrame"))
        (if _returnvalue_3
          (`/Engine/EditorBlueprintResources/StandardMacros.DoOnce` false :!label _label
            (:`Completed`
              ;;;[1 1 1] Marque un tps d'arrêt avant de repartir dans le sens opposé
              (set `CharacterMovementComponent.MaxWalkSpeed` 0.0 (`self.CharacterMovement`))
              (`KismetSystemLibrary.Delay` (`self.WaitTime`))
              (set `CharacterMovementComponent.MaxWalkSpeed` (`self.Max Walk Speed`) (`self.CharacterMovement`))
              (set `self.Direction` (* (`self.Direction`) -1.0))
              (goto _label :!via `Reset`)))))
      (:`then_1`
        ;;[1 1 1] Rotation Vide
        (bind (_outhit_2 _returnvalue_4) (`KismetSystemLibrary.LineTraceSingleForObjects` _returnvalue_2 (+ (- _returnvalue_2 (0.0 0.0 150.0)) (* (`self.GetActorForwardVector`) (50.0 0.0 0.0))) (`|MakeArray` "ObjectTypeQuery1" "ObjectTypeQuery2" "ObjectTypeQuery3" :!type "EObjectTypeQuery Enum") false (`|MakeArray` (`GameplayStatics.GetPlayerCharacter` 0) :!type "Actor Object Reference") "ForOneFrame"))
        (if (not _returnvalue_4)
          (goto _label))))))

(event `self.Box.OnComponentBeginOverlap`
  (params (OverlappedComponent :type "PrimitiveComponent Object Reference") (OtherActor :type "Actor Object Reference") (OtherComp :type "PrimitiveComponent Object Reference") (OtherBodyIndex :type Integer) (bFromSweep :type Boolean) (SweepResult :type "HitResult Structure (by ref)"))
  ;[1 1 1] Système d'ataque
  ;;[1 1 1] Detection du Player
  (if (`self.IsDead`)
    _
    (elif (== OtherActor (`GameplayStatics.GetPlayerCharacter` 0))
      (set `self.AttackMode` true)
      ;;;[1 1 1] Repeter attack toutes les x secondes
      (bind _returnvalue (`KismetSystemLibrary.K2_SetTimerDelegate` (delegate `EnnemyAttack`) 2.0 true -1.5))
      (set `self.AttackEvent` _returnvalue))))

(event `EnnemyAttack`
  ;[1 1 1] Système d'ataque
  ;;[1 1 1] Detection du Player
  ;;;[1 1 1] Repeter attack toutes les x secondes
  (`PaperZDAnimInstance.JumpToNode` (`PaperZDAnimationComponent.AnimInstance` (`self.AnimationComponent`)) "Attacked" "None"))

(event `Attack`
  (bind _returnvalue (`self.K2_GetActorLocation`))
  ;[1 1 1] Système d'ataque
  ;;[1 1 1] Attack
  (bind _outhit (`KismetSystemLibrary.LineTraceSingleForObjects` :`Start` _returnvalue :`End` (+ _returnvalue (* (`self.GetActorForwardVector`) (100.0 0.0 0.0))) :`ObjectTypes` (`|MakeArray` "ObjectTypeQuery3" :!type "EObjectTypeQuery Enum") :`DrawDebugType` "ForDuration"))
  (bind (_bblockinghit _binitialoverlap _time _distance _location _impactpoint _normal _impactnormal _physmat _hitactor) (`GameplayStatics.BreakHitResult` _outhit))
  ;;;[1 1 1] Si l'actor = player alors lui ainfligé dmg
  (if (== _hitactor (`GameplayStatics.GetPlayerCharacter` 0))
    (`GameplayStatics.ApplyDamage` _hitactor 1.0)))

(event `self.ReceiveAnyDamage`
  (params (Damage :type "Float (single-precision)") (DamageType :type "DamageType Object Reference") (InstigatedBy :type "Controller Object Reference") (DamageCauser :type "Actor Object Reference"))
  (bind _returnvalue_x (`KismetMathLibrary.BreakVector` (`KismetMathLibrary.GetDirectionUnitVector` (`self.K2_GetActorLocation` DamageCauser) (`self.K2_GetActorLocation`))))
  (bind _returnvalue (select `bool` (< _returnvalue_x 0.0) :`false` -1.0 :`true` 1.0))
  ;[1 1 1] Hit + Mort
  (if (not (`self.IsDead`))
    ;;[1 1 1] Applique dmg et retire pdv
    (set `self.Health` (- (`self.Health`) Damage))
    (set `self.Damaged` true)
    (set `self.Direction` _returnvalue)
    ;;[1 1 1] Affiche PDV
    (`KismetSystemLibrary.PrintString` (`KismetStringLibrary.Concat_StrStr` "PDV Ennemy : " (`KismetStringLibrary.Conv_DoubleToString` (`self.Health`))) true true (struct :`R` 0.522914 :`B` 1.0 :`A` 1.0))
    ;;[1 1 1] Vérifie si la vie est sup à 0
    (if (<= (`self.Health`) 0.0)
      ;;[1 1 1] Animation mort et détruit l'actor
      (`/Engine/EditorBlueprintResources/StandardMacros.DoOnce` false
        (:`Completed`
          (`PaperZDAnimInstance.JumpToNode` (`PaperZDAnimationComponent.AnimInstance` (`self.AnimationComponent`)) "death" "None")
          (set `self.IsDead` true)
          (`KismetSystemLibrary.K2_ClearAndInvalidateTimerHandle` (`self.AttackEvent`)) ; Reset le TimeEvent
          (`PrimitiveComponent.SetCollisionProfileName` (`self.CapsuleComponent`) "OverlapOnlyPawn" true)
          (`KismetSystemLibrary.Delay` 2.0)
          (`self.K2_DestroyActor`)))
      (else
        ;;[1 1 1] KnockBack + Animation Hit
        (`self.LaunchCharacter` (`KismetMathLibrary.MakeVector` (* _returnvalue -500.0) 0.0 200.0) true true)
        (`PaperZDAnimInstance.JumpToNode` (`PaperZDAnimationComponent.AnimInstance` (`self.AnimationComponent`)) "hited" "None")
        (`KismetSystemLibrary.RetriggerableDelay` 0.5) ; Temps avant reprise move
        (set `self.Damaged` false)))))

(event `self.Box.OnComponentEndOverlap`
  (params (OverlappedComponent :type "PrimitiveComponent Object Reference") (OtherActor :type "Actor Object Reference") (OtherComp :type "PrimitiveComponent Object Reference") (OtherBodyIndex :type Integer))
  ;[1 1 1] Système d'ataque
  ;;[1 1 1] Le player perdu et clear l'event attack
  (if (== OtherActor (`GameplayStatics.GetPlayerCharacter` 0))
    (set `self.AttackMode` false)
    (`KismetSystemLibrary.K2_ClearAndInvalidateTimerHandle` (`self.AttackEvent`)) ; Reset le TimeEvent
  ))

(fn `UserConstructionScript`)