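; BP_EnnemyProject is a ranged enemy character that turns along X to face the player, attacks and takes damage.
; Player overlap with its Box starts a looping timer that jumps the animation state machine to attack.
; A separate Projectile event, not called within this graph, spawns an actor at ProjectilSpawn.
; Damage lowers Health, triggering knockback and a hit animation, or a death animation, collision change and delayed destruction.
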(event `Rotation`
  (bind _returnvalue_x (`KismetMathLibrary.BreakVector` (`KismetMathLibrary.GetDirectionUnitVector` (`self.K2_GetActorLocation` (`GameplayStatics.GetPlayerCharacter` 0)) (`self.K2_GetActorLocation`))))
  ;[1 1 1] Rotation
  (if (not (`self.Is Dead`))
    (if (< _returnvalue_x 0.0)
      (`self.K2_SetActorRotation` (struct))
      (else
        (`self.K2_SetActorRotation` (struct :`Yaw` 180.0))))))

(event `self.ReceiveTick`
  (params (DeltaSeconds :type "Float (single-precision)"))
  (`self.Rotation`))

(event `self.ReceiveAnyDamage`
  (params (Damage :type "Float (single-precision)") (DamageType :type "DamageType Object Reference") (InstigatedBy :type "Controller Object Reference") (DamageCauser :type "Actor Object Reference"))
  (bind _returnvalue_x (`KismetMathLibrary.BreakVector` (`self.GetActorForwardVector`)))
  ;[1 1 1] Hit + Mort
  ;;[1 1 1] Soustraie la vie
  (set `self.Health` (- (`self.Health`) Damage))
  ;;[1 1 1] Affiche PDV
  (`KismetSystemLibrary.PrintString` (`KismetStringLibrary.Concat_StrStr` "PDV Ennemy : " (`KismetStringLibrary.Conv_DoubleToString` (`self.Health`))) true true (struct :`R` 0.522914 :`B` 1.0 :`A` 1.0))
  (if (<= (`self.Health`) 0.0)
    ;;[1 1 1] Animation mort et détruit l'actor
    (`PaperZDAnimInstance.JumpToNode` (`PaperZDAnimationComponent.AnimInstance` (`self.AnimationComponent`)) "death" "None")
    (set `self.Is Dead` true)
    (`PrimitiveComponent.SetCollisionProfileName` (`self.CapsuleComponent`) "OverlapOnlyPawn" true)
    (`KismetSystemLibrary.Delay` 2.0)
    (`self.K2_DestroyActor`)
    (else
      ;;[1 1 1] KnockBack + Animation Hit
      (`self.LaunchCharacter` (`KismetMathLibrary.MakeVector` (* _returnvalue_x -500.0) 0.0 200.0) true true) ; KnockBack
      (`PaperZDAnimInstance.JumpToNode` (`PaperZDAnimationComponent.AnimInstance` (`self.AnimationComponent`)) "damaged" "None"))))

(event `self.Box.OnComponentBeginOverlap`
  (params (OverlappedComponent :type "PrimitiveComponent Object Reference") (OtherActor :type "Actor Object Reference") (OtherComp :type "PrimitiveComponent Object Reference") (OtherBodyIndex :type Integer) (bFromSweep :type Boolean) (SweepResult :type "HitResult Structure (by ref)"))
  ;[1 1 1] Detecte le Player
  (if (== OtherActor (`GameplayStatics.GetPlayerCharacter` 0))
    (`KismetSystemLibrary.K2_SetTimerDelegate` (delegate `Attack`) 2.0 true -1.0)))

(event `Attack`
  ;[1 1 1] Detecte le Player
  (if (not (`self.Is Dead`))
    (`PaperZDAnimInstance.JumpToNode` (`PaperZDAnimationComponent.AnimInstance` (`self.AnimationComponent`)) "attack" "None")))

(event `Projectile`
  ;[1 1 1] Fait Spawn le projectile
  (`|SpawnActorFromClass` null (`KismetMathLibrary.MakeTransform` (`SceneComponent.K2_GetComponentLocation` (`self.ProjectilSpawn`)) (`self.K2_GetActorRotation`)) "Undefined" "MultiplyWithRoot" null null))

(fn `UserConstructionScript`)