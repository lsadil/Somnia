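; Flying enemy, per its name, that turns to face the player along X and periodically attacks while the player is inside its sphere.
; Each tick updates facing unless dead and, if movement is enabled, moves it toward the player along X when within horizontal range.
; Sphere overlaps start and clear a looping timer that jumps the animation to its attack node.
; A separate AttackProjectile event aims the spawn point at the player and spawns an actor.
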(event `self.Sphere.OnComponentBeginOverlap`
  (params (OverlappedComponent :type "PrimitiveComponent Object Reference") (OtherActor :type "Actor Object Reference") (OtherComp :type "PrimitiveComponent Object Reference") (OtherBodyIndex :type Integer) (bFromSweep :type Boolean) (SweepResult :type "HitResult Structure (by ref)"))
  ;[1 1 1] Detecte le Player pour l'attaque
  (if (== OtherActor (`GameplayStatics.GetPlayerCharacter` 0))
    (bind _returnvalue (`KismetSystemLibrary.K2_SetTimerDelegate` (delegate `Attack`) 2.0 true -1.0))
    (set `self.AttackEvent` _returnvalue)))

(event `Rotation`
  (bind _returnvalue_x (`KismetMathLibrary.BreakVector` (`KismetMathLibrary.GetDirectionUnitVector` (`self.K2_GetActorLocation` (`GameplayStatics.GetPlayerCharacter` 0)) (`self.K2_GetActorLocation`))))
  ;[1 1 1] Rotation
  (if (not (`self.Is Dead`))
    (if (< _returnvalue_x 0.0)
      (`self.K2_SetActorRotation` (struct))
      (else
        (`self.K2_SetActorRotation` (struct :`Yaw` 180.0))))))

(event `Attack`
  ;[1 1 1] Detecte le Player pour l'attaque
  (`PaperZDAnimInstance.JumpToNode` (`PaperZDAnimationComponent.AnimInstance` (`self.AnimationComponent`)) "attack" "None"))

(event `self.ReceiveTick`
  (params (DeltaSeconds :type "Float (single-precision)"))
  (bind (_returnvalue_x _returnvalue_y _returnvalue_z) (`KismetMathLibrary.BreakVector` (- (`self.K2_GetActorLocation` (`GameplayStatics.GetPlayerCharacter` 0)) (`self.K2_GetActorLocation`))))
  (bind _returnvalue_x_2 (`KismetMathLibrary.BreakVector` (`KismetMathLibrary.Normal` (`KismetMathLibrary.MakeVector` _returnvalue_x _returnvalue_y _returnvalue_z))))
  ;[1 1 1] Movement
  (`self.Rotation`)
  (if (`self.InMovement?`)
    (if (< (`KismetMathLibrary.Abs` _returnvalue_x) 400.0)
      (`self.AddMovementInput` (1.0 0.0 0.0) _returnvalue_x_2))))

(event `self.Sphere.OnComponentEndOverlap`
  (params (OverlappedComponent :type "PrimitiveComponent Object Reference") (OtherActor :type "Actor Object Reference") (OtherComp :type "PrimitiveComponent Object Reference") (OtherBodyIndex :type Integer))
  ;[1 1 1] Arrete d'attaquer
  (if (== OtherActor (`GameplayStatics.GetPlayerCharacter` 0))
    (`KismetSystemLibrary.K2_ClearAndInvalidateTimerHandle` (`self.AttackEvent`))))

(event `AttackProjectile`
  ;[1 1 1] Projectile
  ;;[1 1 1] Detecte la location du joueur pour ajuster la trajectoire
  (`SceneComponent.K2_SetWorldRotation` (`self.ProjectileSpawn`) (`KismetMathLibrary.FindLookAtRotation` (`self.K2_GetActorLocation`) (`self.K2_GetActorLocation` (`GameplayStatics.GetPlayerCharacter` 0))) false false)
  (`|SpawnActorFromClass` null (`SceneComponent.K2_GetComponentToWorld` (`self.ProjectileSpawn`)) "Undefined" "MultiplyWithRoot" null null))

(fn `UserConstructionScript`)