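; BP_Gato_Intro is a one-shot scripted intro in which a cat falls and walks when BP_Hope enters its box trigger.
; The overlap freezes Hope's movement, first waiting briefly if she is airborne.
; Delays and two chained timelines swap the Paper2D flipbook from fall to walk and drive its world X/Z position.
; Delays chained from the timeline updates then restore Hope's walking movement and destroy the actor.
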(event `self.Box.OnComponentBeginOverlap`
  (params (OverlappedComponent :type "PrimitiveComponent Object Reference") (OtherActor :type "Actor Object Reference") (OtherComp :type "PrimitiveComponent Object Reference") (OtherBodyIndex :type Integer) (bFromSweep :type Boolean) (SweepResult :type "HitResult Structure (by ref)"))
  (bind _paperflipbook (`self.PaperFlipbook`))
  (bind _asbp_hope (cast `/Game/Blueprints/Hope/BP_Hope` OtherActor))
  (`/Engine/EditorBlueprintResources/StandardMacros.DoOnce` false
    (:`Completed`
      (bind _charactermovement (`Character.CharacterMovement` _asbp_hope))
      (if (`NavMovementComponent.IsFalling` _charactermovement)
        (set `CharacterMovementComponent.AirControl` 0.0 _charactermovement)
        (set `CharacterMovementComponent.MaxWalkSpeed` 0.0 _charactermovement)
        (`KismetSystemLibrary.Delay` 1.3))
      (`CharacterMovementComponent.DisableMovement` _charactermovement)
      (`KismetSystemLibrary.Delay` 0.5)
      (`PaperFlipbookComponent.SetFlipbook` (`self.PaperFlipbook`) "/Game/Assets/NPC/Gato/Fall/FB_Cato_fall.FB_Cato_fall")
      (`SceneComponent.K2_SetRelativeRotation` (`self.PaperFlipbook`) (struct :`Yaw` 180.0) false false)
      (`KismetSystemLibrary.Delay` 0.4)
      (bind (_direction _newtrack_0 _newtrack_1) (`Timeline|Timeline`)
        (:`Update`
          (`SceneComponent.K2_SetWorldLocation` _paperflipbook (`KismetMathLibrary.MakeVector` _newtrack_0 0.0 _newtrack_1) false false)
          (`KismetSystemLibrary.Delay` 0.7)
          (`PaperFlipbookComponent.SetFlipbook` _paperflipbook "/Game/Assets/NPC/Gato/Walk/FB_gato_walk_red.FB_gato_walk_red")
          (bind (_direction_2 _newtrack_0_2) (`Timeline|Timeline_0`)
            (:`Update`
              (`SceneComponent.K2_SetWorldLocation` (`self.PaperFlipbook`) (`KismetMathLibrary.MakeVector` _newtrack_0_2 0.0 -445.0) false false)
              (`KismetSystemLibrary.Delay` 2.8)
              (bind _asbp_hope_2 (cast `/Game/Blueprints/Hope/BP_Hope` (`GameplayStatics.GetPlayerCharacter` 0)))
              (bind _charactermovement_2 (`Character.CharacterMovement` _asbp_hope_2))
              (set `CharacterMovementComponent.AirControl` 1.0 _charactermovement_2)
              (set `CharacterMovementComponent.MaxWalkSpeed` 650.0 _charactermovement_2)
              (`CharacterMovementComponent.SetMovementMode` _charactermovement_2 "MOVE_Walking" 0)
              (`KismetSystemLibrary.Delay` 0.1)
              (`self.K2_DestroyActor`))))))))

(fn `UserConstructionScript`)