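; Actor component that makes a given actor follow a BP_MagicSpell_Tornado along the X axis.
; TornadoCollision stores the actor, prints a debug message, loops over all tornado actors and sets a detection flag that is never cleared here.
; Tick then teleport-free sets the actor's transform every frame, using the last looped tornado's X, rotation and scale while keeping its own Y and Z.
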(event `TornadoCollision`
  (params (ActorRef :type "Actor Object Reference"))
  (set `self.Actor Ref` ActorRef)
  (`/Engine/EditorBlueprintResources/StandardMacros.IsValid` "/Game/Blueprints/Runes/Runes_MagicSpells/BP_MagicSpell_Tornado.BP_MagicSpell_Tornado"
    (:`Is Valid`
      (`KismetSystemLibrary.PrintString` "TornadoDetected")
      (bind _outactors (`GameplayStatics.GetAllActorsOfClass` "/Game/Blueprints/Runes/Runes_MagicSpells/BP_MagicSpell_Tornado.BP_MagicSpell_Tornado_C"))
      (for _array_element _outactors
        (set `self.ActorDetected` true)))))

(event `self.ReceiveTick`
  (params (DeltaSeconds :type "Float (single-precision)"))
  (bind (_returnvalue_x _returnvalue_y _returnvalue_z) (`KismetMathLibrary.BreakVector` (`Actor.K2_GetActorLocation` (`self.Actor Ref`))))
  (if (`self.ActorDetected`)
    (`/Engine/EditorBlueprintResources/StandardMacros.IsValid` (stale `TornadoCollision` _array_element)
      (:`Is Valid`
        (bind _returnvalue (`Actor.GetTransform` (stale `TornadoCollision` _array_element)))
        (set `self.ActorTransform` (`KismetMathLibrary.MakeTransform` (`KismetMathLibrary.MakeVector` (.x (.location _returnvalue)) _returnvalue_y _returnvalue_z) (.rotation _returnvalue) (.scale _returnvalue)))
        (`Actor.K2_SetActorTransform` (`self.Actor Ref`) (`self.ActorTransform`) false false)))))