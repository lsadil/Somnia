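; BP_DamageZone is a box trigger that damages an overlapping actor on entry and repeatedly while it stays inside.
; Begin overlap applies Damage immediately and starts a looping timer at Cooldown intervals; end overlap clears it.
; A single timer handle and the latest overlap's OtherActor drive the damage, so overlapping actors are not tracked separately.
; The construction script assigns the configurable sprite and flipbook when Sprite is valid.
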(event `self.Box.OnComponentBeginOverlap`
  (params (OverlappedComponent :type "PrimitiveComponent Object Reference") (OtherActor :type "Actor Object Reference") (OtherComp :type "PrimitiveComponent Object Reference") (OtherBodyIndex :type Integer) (bFromSweep :type Boolean) (SweepResult :type "HitResult Structure (by ref)"))
  (`self.Apply Damage`)
  (bind _returnvalue (`KismetSystemLibrary.K2_SetTimerDelegate` (delegate `Apply Damage`) (`self.Cooldown`) true))
  (set `self.Timer` _returnvalue))

(event `Apply Damage`
  (`GameplayStatics.ApplyDamage` (stale `self.Box.OnComponentBeginOverlap` OtherActor) (`self.Damage`)))

(event `self.Box.OnComponentEndOverlap`
  (params (OverlappedComponent :type "PrimitiveComponent Object Reference") (OtherActor :type "Actor Object Reference") (OtherComp :type "PrimitiveComponent Object Reference") (OtherBodyIndex :type Integer))
  (`KismetSystemLibrary.K2_ClearAndInvalidateTimerHandle` (`self.Timer`)))

(fn `UserConstructionScript`
  (bind _sprite (`self.Sprite`))
  (`/Engine/EditorBlueprintResources/StandardMacros.IsValid` _sprite
    (:`Is Valid`
      (`PaperSpriteComponent.SetSprite` (`self.PaperSprite`) _sprite)
      (`PaperFlipbookComponent.SetFlipbook` (`self.PaperFlipbook`) (`self.Flipbook`)))))