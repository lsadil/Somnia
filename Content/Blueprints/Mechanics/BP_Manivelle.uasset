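; Crank actor (manivelle) that moves a linked Platform between its start location and an X/Z offset while the player operates it.
; Interact and Stop toggle rotation, which also requires the player to be inside the Box overlap.
; While active, Tick spins the Paper sprite and plays a Timeline that lerps the platform's root.
; Otherwise, Tick reverses the Timeline after a delay, returning the platform.
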(event `self.ReceiveBeginPlay`
  (bind _output_get (set `self.Start Location` (`self.K2_GetActorLocation` (`self.Platform`))))
  (set `self.End Location` (`KismetMathLibrary.MakeVector` (+ (`self.End Location X`) (.x _output_get)) (.y _output_get) (+ (.z _output_get) (`self.End Location Z`))))
  (set `self.Done` false))

(event `self.ReceiveTick`
  (params (DeltaSeconds :type "Float (single-precision)"))
  (if (and (`self.Rotating?`) (`self.In Range`))
    (`SceneComponent.K2_AddLocalRotation` (`self.PaperSprite`) (`KismetMathLibrary.MakeRotator` 0.0 (* DeltaSeconds (`self.Rotation`))) false false)
    (bind (_direction _newtrack_2) (`Timeline|Timeline` :!label _label)
      (:`Update`
        (`SceneComponent.K2_SetRelativeLocation` (`Actor.RootComponent` (`self.Platform`)) (`KismetMathLibrary.VLerp` (`self.Start Location`) (`self.End Location`) _newtrack_2) false false)))
    (else
      (`KismetSystemLibrary.Delay` (`self.Delay Duration`))
      (goto _label :!via `Reverse`))))

(event `/Game/Blueprints/Interfaces/BPI_Interact.Interact`
  (set `self.Rotating?` true))

(event `/Game/Blueprints/Interfaces/BPI_Interact.Stop`
  (set `self.Rotating?` false))

(event `self.Box.OnComponentBeginOverlap`
  (params (OverlappedComponent :type "PrimitiveComponent Object Reference") (OtherActor :type "Actor Object Reference") (OtherComp :type "PrimitiveComponent Object Reference") (OtherBodyIndex :type Integer) (bFromSweep :type Boolean) (SweepResult :type "HitResult Structure (by ref)"))
  (if (== OtherActor (`GameplayStatics.GetPlayerCharacter` 0))
    (set `self.In Range` true)))

(event `self.Box.OnComponentEndOverlap`
  (params (OverlappedComponent :type "PrimitiveComponent Object Reference") (OtherActor :type "Actor Object Reference") (OtherComp :type "PrimitiveComponent Object Reference") (OtherBodyIndex :type Integer))
  (if (== OtherActor (`GameplayStatics.GetPlayerCharacter` 0))
    (set `self.In Range` false)))

(fn `UserConstructionScript`)