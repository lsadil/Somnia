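; BP_Manivelle1 is a crank that the player character (BP_Hope) turns to move a linked platform.
; Interact and Stop toggle the rotating state and Hope's Interacting flag, with Interact also starting a rail sound, while a box overlap tracks range.
; While rotating in range, Tick spins the sprite and plays a timeline lerping the platform between start and end locations.
; Otherwise, the timeline reverses after a delay.
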(event `self.ReceiveBeginPlay`
  (set `self.Done` false)
  (bind _asbp_hope (cast `/Game/Blueprints/Hope/BP_Hope` (`GameplayStatics.GetPlayerCharacter` 0)))
  (set `self.Hope` _asbp_hope))

(event `/Game/Blueprints/Interfaces/BPI_Interact.Interact`
  (bind _audio (`self.Audio`))
  (set `self.Rotating?` true)
  (set `/Game/Blueprints/Hope/BP_Hope.Interacting?` true (`self.Hope`))
  (`AudioComponent.SetSound` _audio "/Game/Assets/SD/SFXQ/UI/SFX_RAILS_MID_Cue.SFX_RAILS_MID_Cue")
  (`AudioComponent.Play` _audio 0.0))

(event `self.ReceiveTick`
  (params (DeltaSeconds :type "Float (single-precision)"))
  (if (and (`self.Rotating?`) (`self.In Range`))
    (`SceneComponent.K2_AddLocalRotation` (`self.PaperSprite`) (`KismetMathLibrary.MakeRotator` 0.0 (* DeltaSeconds (`self.Rotation`))) false false)
    (bind (_direction _newtrack_2) (`Timeline|Timeline` :!label _label)
      (:`Update`
        (`SceneComponent.K2_SetRelativeLocation` (`Actor.RootComponent` (`self.Platform`)) (`KismetMathLibrary.VLerp` (`self.Start Location`) (`self.End Location`) _newtrack_2) false false)))
    (else
      (`KismetSystemLibrary.Delay` (`self.Delay Duration`))
      (goto _label :!via `Reverse`))))

(event `/Game/Blueprints/Interfaces/BPI_Interact.Stop`
  (set `self.Rotating?` false)
  (set `/Game/Blueprints/Hope/BP_Hope.Interacting?` false (`self.Hope`))
  (`AudioComponent.SetPaused` (`self.Audio`) false))

(event `self.Box.OnComponentBeginOverlap`
  (params (OverlappedComponent :type "PrimitiveComponent Object Reference") (OtherActor :type "Actor Object Reference") (OtherComp :type "PrimitiveComponent Object Reference") (OtherBodyIndex :type Integer) (bFromSweep :type Boolean) (SweepResult :type "HitResult Structure (by ref)"))
  (if (== OtherActor (`GameplayStatics.GetPlayerCharacter` 0))
    (set `self.In Range` true)))

(event `self.Box.OnComponentEndOverlap`
  (params (OverlappedComponent :type "PrimitiveComponent Object Reference") (OtherActor :type "Actor Object Reference") (OtherComp :type "PrimitiveComponent Object Reference") (OtherBodyIndex :type Integer))
  (if (== OtherActor (`GameplayStatics.GetPlayerCharacter` 0))
    (set `self.In Range` false)))

(fn `UserConstructionScript`)