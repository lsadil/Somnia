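; BP_ObjTornado is a world object that reacts to being hit by the tornado magic spell.
; The construction script sets its paper sprite to the default sprite.
; When its box overlaps a BP_MagicSpell_Tornado actor, it passes itself to the ACCollisionTornado component's TornadoCollision and swaps to a second sprite.
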(event `self.Box.OnComponentBeginOverlap`
  (params (OverlappedComponent :type "PrimitiveComponent Object Reference") (OtherActor :type "Actor Object Reference") (OtherComp :type "PrimitiveComponent Object Reference") (OtherBodyIndex :type Integer) (bFromSweep :type Boolean) (SweepResult :type "HitResult Structure (by ref)"))
  (if (== (`GameplayStatics.GetObjectClass` OtherActor) "/Game/Blueprints/Runes/Runes_MagicSpells/BP_MagicSpell_Tornado.BP_MagicSpell_Tornado_C")
    (`/Game/Blueprints/Mechanics/AC_CollisionTornado.TornadoCollision` (`self.AC_CollisionTornado`) self)
    (`PaperSpriteComponent.SetSprite` (`self.PaperSprite`) (`self.Sprite2`))))

(fn `UserConstructionScript`
  (`PaperSpriteComponent.SetSprite` (`self.PaperSprite`) (`self.Sprite`)))