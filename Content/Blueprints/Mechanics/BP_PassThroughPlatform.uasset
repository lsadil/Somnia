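; One-way platform that the player can pass through and drop down from.
; Each tick a Z-value gate sets the box's response on a game trace channel to Ignore, or to Block if CanDropDown is set.
; PlayerDropDown briefly forces Ignore, with Tick updates suspended while the player overlaps the range sphere.
; The construction script sizes box and sphere from the sprite-count length and disables sprite collision.
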(event `self.ReceiveTick`
  (params (DeltaSeconds :type "Float (single-precision)"))
  (bind (_returnvalue_x _returnvalue_y _returnvalue_z) (`KismetMathLibrary.BreakVector` (`self.K2_GetActorLocation`)))
  (bind (_returnvalue_x_2 _returnvalue_y_2 _returnvalue_z_2) (`KismetMathLibrary.BreakVector` (`self.K2_GetActorLocation` (`GameplayStatics.GetPlayerCharacter` 0))))
  (if (and (`self.DroppingDown`) (`self.PlayerInRange`))
    _
    (elif (< _returnvalue_z_2 (+ _returnvalue_z 30.0))
      (`PrimitiveComponent.SetCollisionResponseToChannel` (`self.Box`) "ECC_GameTraceChannel1" "ECR_Ignore")
      (elif (`self.Can Drop Down`)
        (`PrimitiveComponent.SetCollisionResponseToChannel` (`self.Box`) "ECC_GameTraceChannel1" "ECR_Block")))))

(event `self.Sphere.OnComponentBeginOverlap`
  (params (OverlappedComponent :type "PrimitiveComponent Object Reference") (OtherActor :type "Actor Object Reference") (OtherComp :type "PrimitiveComponent Object Reference") (OtherBodyIndex :type Integer) (bFromSweep :type Boolean) (SweepResult :type "HitResult Structure (by ref)"))
  (if (== OtherActor (`GameplayStatics.GetPlayerCharacter` 0))
    (set `self.PlayerInRange` true)))

(event `self.Sphere.OnComponentEndOverlap`
  (params (OverlappedComponent :type "PrimitiveComponent Object Reference") (OtherActor :type "Actor Object Reference") (OtherComp :type "PrimitiveComponent Object Reference") (OtherBodyIndex :type Integer))
  (if (== OtherActor (`GameplayStatics.GetPlayerCharacter` 0))
    (set `self.PlayerInRange` false)))

(event `/Game/Blueprints/Interfaces/BPI_Interact.PlayerDropDown`
  (set `self.DroppingDown` true)
  (`PrimitiveComponent.SetCollisionResponseToChannel` (`self.Box`) "ECC_GameTraceChannel1" "ECR_Ignore")
  (`KismetSystemLibrary.Delay` 0.3)
  (set `self.DroppingDown` false))

(fn `Interact`
  (return))

(fn `UserConstructionScript`
  (bind _returnvalue (* (+ (`self.PlatfromLengthInSprites`) 1) 8.0))
  (`BoxComponent.SetBoxExtent` (`self.Box`) (`KismetMathLibrary.MakeVector` _returnvalue 40.0 8.0) true)
  (`SphereComponent.SetSphereRadius` (`self.Sphere`) (* _returnvalue 2.0) true)
  (for _array_element (`self.Sprites`)
    (`PrimitiveComponent.SetCollisionEnabled` _array_element "NoCollision")))