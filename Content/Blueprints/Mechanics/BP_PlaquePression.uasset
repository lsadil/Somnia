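; BP_PlaquePression is a pressure plate that toggles on or off each time BP_Hope begins overlapping its box.
; Each press flips State and swaps the plate's Paper2D sprite between on and off, starting from off at construction.
; The same press sets the referenced PictoActor's sprite from PictoSpritesArray, using a counter that wraps around to cycle through the pictograms.
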(event `self.Box.OnComponentBeginOverlap`
  (params (OverlappedComponent :type "PrimitiveComponent Object Reference") (OtherActor :type "Actor Object Reference") (OtherComp :type "PrimitiveComponent Object Reference") (OtherBodyIndex :type Integer) (bFromSweep :type Boolean) (SweepResult :type "HitResult Structure (by ref)"))
  (cast `/Game/Blueprints/Hope/BP_Hope` OtherActor)
  (`self.Switch State`)
  (`self.Switch Picto`))

(fn `Switch Picto`
  (`PaperSpriteComponent.SetSprite` (`/Game/Blueprints/Mechanics/BP_PictoActor.PaperSprite` (`self.PictoActor`)) (`|GetArrayItem` (`self.Picto Sprites Array`) (`self.Count`)))
  (bind _result (`/Engine/EditorBlueprintResources/StandardMacros.IncrementInt` (`self.Count`))
    (:`  `
      (set `self.Count` (mod _result (`KismetArrayLibrary.Array_Length` (`self.Picto Sprites Array`)))))))

(fn `Switch State`
  (returns (State :type Boolean))
  (bind _output_get (set `self.State` (not (`self.State`))))
  (if _output_get
    (`PaperSpriteComponent.SetSprite` (`self.PaperSprite`) (`self.SpriteOn`))
    (return true)
    (else
      (`PaperSpriteComponent.SetSprite` (`self.PaperSprite`) (`self.SpriteOff`))
      (return false))))

(fn `UserConstructionScript`
  (`PaperSpriteComponent.SetSprite` (`self.PaperSprite`) (`self.SpriteOff`)))