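; Interactable Paper2D switch that toggles on and off to move a referenced object between two locations.
; Each interaction flips the state, swaps the switch sprite, and plays or reverses a Timeline accordingly.
; The Timeline lerps the object's root component from its location, captured in the Construction Script, to an end location, without sweeping.
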(event `/Game/Blueprints/Interfaces/BPI_Interact.Interact`
  (bind _state (`self.Switch State`))
  (if _state
    (bind (_direction _newtrack_0) (`Timeline|Timeline` :!label _label)
      (:`Update`
        (`SceneComponent.K2_SetRelativeLocation` (`Actor.RootComponent` (`self.Object`)) (`KismetMathLibrary.VLerp` (`self.Start Location`) (`self.End Location`) _newtrack_0) false false)))
    (else
      (goto _label :!via `Reverse`))))

(fn `Switch State`
  (returns (State :type Boolean))
  (bind _output_get (set `self.State` (not (`self.State`))))
  (if _output_get
    (`PaperSpriteComponent.SetSprite` (`self.PaperSprite`) null)
    (return true)
    (else
      (`PaperSpriteComponent.SetSprite` (`self.PaperSprite`) null)
      (return false))))

(fn `UserConstructionScript`
  (set `self.Start Location` (`self.K2_GetActorLocation` (`self.Object`))))