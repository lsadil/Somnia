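; BP_Tornado_Switch is a switch triggered by TornadoInteract that moves a Target actor between a start and end location.
; The result of SwitchState picks whether a timeline plays forward or reverses, lerping the Target's root component relative location.
; A DoOnce blocks retriggering until the timeline finishes.
; The plain Interact event is empty, so that interaction does nothing here.
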(event `/Game/Blueprints/Interfaces/BPI_Interact.Tornado Interact`
  (`/Engine/EditorBlueprintResources/StandardMacros.DoOnce` false :!label _label
    (:`Completed`
      (bind _state (`self.Switch State`))
      (if _state
        (bind (_direction _newtrack_0) (`Timeline|Timeline_0` :!label _label_2)
          (:`Update`
            (`SceneComponent.K2_SetRelativeLocation` (`Actor.RootComponent` (`self.Target`)) (`KismetMathLibrary.VLerp` (`self.Start Location`) (`self.End Location`) _newtrack_0) false false))
          (:`Finished`
            (goto _label :!via `Reset`)))
        (else
          (goto _label_2 :!via `Reverse`))))))

(event `/Game/Blueprints/Interfaces/BPI_Interact.Interact`)

(fn `UserConstructionScript`
  (`parent.UserConstructionScript`))