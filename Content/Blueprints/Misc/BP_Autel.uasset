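; BP_Autel is an altar actor that unlocks either the staff or the tornado for BP_Hope when that character overlaps its Box.
; The StaffTornado boolean selects the reward, setting HasStaff when true and HasTornado when false on the overlapping character.
; The construction script shows FlipbookOff on the Sprite if valid, and the overlap swaps it to Flipbook, with no reset in the graph.
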(event `self.Box.OnComponentBeginOverlap`
  (params (OverlappedComponent :type "PrimitiveComponent Object Reference") (OtherActor :type "Actor Object Reference") (OtherComp :type "PrimitiveComponent Object Reference") (OtherBodyIndex :type Integer) (bFromSweep :type Boolean) (SweepResult :type "HitResult Structure (by ref)"))
  (bind _asbp_hope (cast `/Game/Blueprints/Hope/BP_Hope` OtherActor))
  (if (`self.Staff? : Tornado`)
    (set `/Game/Blueprints/Hope/BP_Hope.HasStaff` true _asbp_hope)
    (else
      (set `/Game/Blueprints/Hope/BP_Hope.HasTornado` true _asbp_hope)))
  (`PaperFlipbookComponent.SetFlipbook` (`self.Sprite`) (`self.Flipbook`)))

(fn `UserConstructionScript`
  (bind _flipbookoff (`self.FlipbookOff`))
  (`/Engine/EditorBlueprintResources/StandardMacros.IsValid` _flipbookoff
    (:`Is Valid`
      (`PaperFlipbookComponent.SetFlipbook` (`self.Sprite`) _flipbookoff))))