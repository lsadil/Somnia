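; BP_StartStop_Music is a trigger actor that starts music on overlap and stops it when the overlap ends.
; An actor overlap spawns an editor-chosen 2D sound and stores it, while Box begin and end overlaps play it from the start or stop it.
; Overlaps only check that player character 0 exists, and a text render shows a label set on BeginPlay.
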(event `self.ReceiveBeginPlay`
  (`TextRenderComponent.K2_SetText` (`self.TextRender`) (`self.Texte`)))

(event `self.ReceiveActorBeginOverlap`
  (params (OtherActor :type "Actor Object Reference"))
  (`/Engine/EditorBlueprintResources/StandardMacros.IsValid` (`GameplayStatics.GetPlayerCharacter` 0)
    (:`Is Valid`
      (bind _returnvalue (`GameplayStatics.SpawnSound2D` (`self.MusicEditorChoice`) 1.0 1.0 0.0 null))
      (set `self.SoundRef` _returnvalue))))

(event `self.Box.OnComponentBeginOverlap`
  (params (OverlappedComponent :type "PrimitiveComponent Object Reference") (OtherActor :type "Actor Object Reference") (OtherComp :type "PrimitiveComponent Object Reference") (OtherBodyIndex :type Integer) (bFromSweep :type Boolean) (SweepResult :type "HitResult Structure (by ref)"))
  (bind _soundref (`self.SoundRef`))
  (`/Engine/EditorBlueprintResources/StandardMacros.IsValid` (`GameplayStatics.GetPlayerCharacter` 0)
    (:`Is Valid`
      (bind _output_get (set `self.isPlayerTriggering` true))
      (`KismetSystemLibrary.PrintString` (`KismetStringLibrary.Conv_BoolToString` _output_get))
      (`/Engine/EditorBlueprintResources/StandardMacros.IsValid` _soundref
        (:`Is Valid`
          (`AudioComponent.Play` _soundref 0.0))))))

(event `self.Box.OnComponentEndOverlap`
  (params (OverlappedComponent :type "PrimitiveComponent Object Reference") (OtherActor :type "Actor Object Reference") (OtherComp :type "PrimitiveComponent Object Reference") (OtherBodyIndex :type Integer))
  (bind _soundref (`self.SoundRef`))
  (`/Engine/EditorBlueprintResources/StandardMacros.IsValid` (`GameplayStatics.GetPlayerCharacter` 0)
    (:`Is Valid`
      (bind _output_get (set `self.isPlayerTriggering` false))
      (`KismetSystemLibrary.PrintString` (`KismetStringLibrary.Conv_BoolToString` _output_get))
      (`/Engine/EditorBlueprintResources/StandardMacros.IsValid` _soundref
        (:`Is Valid`
          (`AudioComponent.Stop` _soundref))))))

(fn `UserConstructionScript`)