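; Trampoline platform that launches the player character upward when they enter its trigger box.
; A guarded overlap plays a timeline that dips the cube, then launches after a short delay, overriding all velocity axes so horizontal momentum is cancelled.
; OnHitMarteau (hammer hit) briefly raises the launch strength before setting it back.
; The collision-toggling logic intended for the other box is disconnected and never runs.
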(event `self.ReceiveBeginPlay`)

(event `self.Box.OnComponentBeginOverlap`
  (params (OverlappedComponent :type "PrimitiveComponent Object Reference") (OtherActor :type "Actor Object Reference") (OtherComp :type "PrimitiveComponent Object Reference") (OtherBodyIndex :type Integer) (bFromSweep :type Boolean) (SweepResult :type "HitResult Structure (by ref)"))
  ;[1 1 1] Active collision
)

(event `self.Box.OnComponentEndOverlap`
  (params (OverlappedComponent :type "PrimitiveComponent Object Reference") (OtherActor :type "Actor Object Reference") (OtherComp :type "PrimitiveComponent Object Reference") (OtherBodyIndex :type Integer))
  ;[1 1 1] Désactive collision
)

(event `self.Box1.OnComponentBeginOverlap`
  (params (OverlappedComponent :type "PrimitiveComponent Object Reference") (OtherActor :type "Actor Object Reference") (OtherComp :type "PrimitiveComponent Object Reference") (OtherBodyIndex :type Integer) (bFromSweep :type Boolean) (SweepResult :type "HitResult Structure (by ref)"))
  (bind _returnvalue (`GameplayStatics.GetPlayerCharacter` 0))
  ;[1 1 1] Active Trmp
  (if (== OtherActor _returnvalue)
    (`/Engine/EditorBlueprintResources/StandardMacros.DoOnce` false :!label _label
      (:`Completed`
        (`self.Trampo`)
        (`KismetSystemLibrary.RetriggerableDelay` 0.3)
        (`Character.LaunchCharacter` _returnvalue (`KismetMathLibrary.MakeVector` 0.0 0.0 (`self.test`)) true true)
        (goto _label :!via `Reset`)))))

(event `Trampo`
  ;[1 1 1] Trampo
  (bind (_direction _newtrack_0) (`Timeline|Timeline_0` :!via `PlayFromStart`)
    (:`Update`
      (`SceneComponent.K2_SetRelativeLocation` (`self.Cube`) (`KismetMathLibrary.MakeVector` 0.0 0.0 (`KismetMathLibrary.Lerp` 0.0 -50.0 _newtrack_0)) false false))))

(event `self.OnHitMarteau`
  (set `self.test` 1250.0)
  (`KismetSystemLibrary.Delay` 0.5)
  (set `self.test` 750.0))

(fn `UserConstructionScript`)