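; BP_Hammer is a hammer rune attack that deals area damage around the player.
; Its Attack event finds BP_Hope and calls HammerAttack on it.
; A separate AOEMarteau event, guarded by a DoOnce, applies full radial damage centered on the player character, who is ignored, plays a camera shake there, then destroys the hammer actor.
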(event `AOE Marteau`
  (bind _returnvalue (`GameplayStatics.GetPlayerCharacter` 0))
  (bind _returnvalue_2 (`self.K2_GetActorLocation` _returnvalue))
  ;[1 1 1] AOE
  (`/Engine/EditorBlueprintResources/StandardMacros.DoOnce` false
    (:`Completed`
      (`GameplayStatics.ApplyRadialDamage` 1.0 _returnvalue_2 300.0 null (`|MakeArray` _returnvalue :!type "Actor Object Reference") self null true)
      (`GameplayStatics.PlayWorldCameraShake` "/Game/Blueprints/Runes/Runes_Attacks/MarteauSkake.MarteauSkake_C" _returnvalue_2 0.0 1500.0)
      (`self.K2_DestroyActor`))))

(event `/Game/Blueprints/Interfaces/BPI_Attack.Attack`
  ;[1 1 1] Call l'attack dans le bp hope
  (bind _returnvalue (`GameplayStatics.GetActorOfClass` "/Game/Blueprints/Hope/BP_Hope.BP_Hope_C"))
  (bind _asbp_hope (cast `/Game/Blueprints/Hope/BP_Hope` _returnvalue))
  (`/Game/Blueprints/Hope/BP_Hope.HammerAttack` _asbp_hope))

(fn `UserConstructionScript`
  (`parent.UserConstructionScript`))