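; Chargeable tornado rune spell, shown as a flipbook, that travels forward from the caster on key release.
; Tick tracks hold time through a gate opened on press, destroying the spell if overcharged.
; Release picks normal or charged state, applies X-only recoil to the player, sweeps the actor by timeline lerp and sets a short lifespan.
; Box overlaps send TornadoInteractMessage to actors implementing BPI_Interact.
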(event `self.ReceiveTick`
  (params (DeltaSeconds :type "Float (single-precision)"))
  (bind _loadtornadosound (`self.LoadTornadoSound`))
  (`parent.ReceiveTick` DeltaSeconds)
  (if (>= (`self.TimeKeyDown`) 3.0)
    (`/Engine/EditorBlueprintResources/StandardMacros.IsValid` _loadtornadosound
      (:`Is Valid`
        (`AudioComponent.Stop` _loadtornadosound))
      (:`Is Not Valid`
        _))
    (`self.K2_DestroyActor`)
    (else
      ;[1 1 1] Event Pressed
      (`/Engine/EditorBlueprintResources/StandardMacros.Gate` true :!label _label
        (:`Exit`
          (bind _output_get (set `self.TimeKeyDown` (`PlayerController.GetInputKeyTimeDown` (`GameplayStatics.GetPlayerController` 0) (stale `/Game/Blueprints/Interfaces/BPI_Spell_Magic.Pressed` Key)))))))))

(event `/Game/Blueprints/Interfaces/BPI_Spell_Magic.Pressed`
  (params (Transform :type "Transform Structure") (Key :type "Key Structure") (ForwardVector :type "Vector Structure"))
  (bind _tornado (`self.Tornado`))
  ;[1 1 1] Event Pressed
  (bind _returnvalue (`GameplayStatics.SpawnSound2D` "/Game/Assets/SD/SFXQ/Tornade/SC_Tornado_Load.SC_Tornado_Load" 1.0 1.0 0.0 null))
  (set `self.LoadTornadoSound` _returnvalue)
  (set `self.Forward Vector` ForwardVector)
  (set `self.Player Transform` Transform)
  (`PaperFlipbookComponent.SetFlipbook` _tornado "/Game/Assets/Runes/Tornado/NewFolder/FB_tr.FB_tr")
  (`PaperFlipbookComponent.Play` _tornado)
  (`AudioComponent.Play` (`self.LoadTornadoSound`) 0.0)
  (goto _label :!via `Open`))

(event `/Game/Blueprints/Interfaces/BPI_Spell_Magic.Released`
  (bind _returnvalue (`GameplayStatics.GetPlayerCharacter` 0))
  (bind _releasedtornadosound (`self.ReleasedTornadoSound`))
  (bind _loadtornadosound (`self.LoadTornadoSound`))
  ;[1 1 1] Event Released
  (`/Engine/EditorBlueprintResources/StandardMacros.IsValid` _loadtornadosound
    (:`Is Valid`
      (`AudioComponent.FadeOut` _loadtornadosound 0.5 0.0 "Linear")
      (bind _returnvalue_2 (`GameplayStatics.SpawnSound2D` "/Game/Assets/SD/SFXQ/Tornade/SC_Tornado_Shot.SC_Tornado_Shot" 1.5 1.0 0.0 null))
      (set `self.ReleasedTornadoSound` _returnvalue_2)
      (`KismetSystemLibrary.PrintString` "Released from BP_MS")
      (`|ExecutionSequence`
        (:`then_0`
          (goto _label :!via `Close`))
        (:`then_1`
          (`self.TimeStateTornado`)
          (`Character.LaunchCharacter` _returnvalue (* (`self.GetActorForwardVector` _returnvalue) (-500.0 0.0 0.0)) false false)
          (bind _transform (`self.LaunchTornado`))
          (bind _output_get (set `self.Transform Location` (.location _transform)))
          (`AudioComponent.Play` (`self.ReleasedTornadoSound`) 0.0)
          (if (`self.TornadoOverload`)
            _
            (elif (`self.isTornadoCharged?`)
              (bind (_direction _0_1) (`Timeline|TwoSec`)
                (:`Update`
                  (bind _returnvalue_3 (`KismetMathLibrary.MakeTransform` _output_get))
                  (`SceneComponent.K2_SetWorldTransform` (`self.DefaultSceneRoot`) (`KismetMathLibrary.TLerp` (`self.Player Transform`) _returnvalue_3 _0_1) true false))
                (:`Finished`
                  (`self.SetLifeSpan` 0.5 :!label _label_2)
                  (`/Engine/EditorBlueprintResources/StandardMacros.IsValid` _releasedtornadosound
                    (:`Is Valid`
                      (`AudioComponent.FadeOut` _releasedtornadosound 1.0 0.0 "Linear")))))
              (else
                (bind (_direction_2 _0_1_2) (`Timeline|OneSec`)
                  (:`Update`
                    (`SceneComponent.K2_SetWorldTransform` (`self.DefaultSceneRoot`) (`KismetMathLibrary.TLerp` (`self.Player Transform`) _returnvalue_3 _0_1_2) true false))
                  (:`Finished`
                    (goto _label_2)))))))))
    (:`Is Not Valid`
      (`KismetSystemLibrary.PrintString` "Not valid"))))

(event `self.Box.OnComponentHit`
  (params (HitComponent :type "PrimitiveComponent Object Reference") (OtherActor :type "Actor Object Reference") (OtherComp :type "PrimitiveComponent Object Reference") (NormalImpulse :type "Vector Structure") (Hit :type "HitResult Structure (by ref)"))
  (`/Engine/EditorBlueprintResources/StandardMacros.IsValid` "/Game/Blueprints/Enemy1/BP_Enemy1.BP_Enemy1"
    (:`Is Valid`
      (`KismetSystemLibrary.PrintString` "Enemy"))))

(event `self.Tornado.OnComponentBeginOverlap`
  (params (OverlappedComponent :type "PrimitiveComponent Object Reference") (OtherActor :type "Actor Object Reference") (OtherComp :type "PrimitiveComponent Object Reference") (OtherBodyIndex :type Integer) (bFromSweep :type Boolean) (SweepResult :type "HitResult Structure (by ref)")))

(event `self.Box.OnComponentBeginOverlap`
  (params (OverlappedComponent :type "PrimitiveComponent Object Reference") (OtherActor :type "Actor Object Reference") (OtherComp :type "PrimitiveComponent Object Reference") (OtherBodyIndex :type Integer) (bFromSweep :type Boolean) (SweepResult :type "HitResult Structure (by ref)"))
  ;[1 1 1] Interaction
  (`KismetSystemLibrary.PrintString` "Hello")
  (if (`KismetSystemLibrary.DoesImplementInterface` OtherActor "/Game/Blueprints/Interfaces/BPI_Interact.BPI_Interact_C")
    (message `/Game/Blueprints/Interfaces/BPI_Interact.Tornado Interact` OtherActor)))

(fn `LaunchTornado`
  (returns (Transform :type "Transform Structure"))
  (bind _player_transform_location (`KismetMathLibrary.BreakTransform` (`self.Player Transform`)))
  (bind _player_transform_location_2 (`KismetMathLibrary.BreakTransform` (`self.Player Transform`)))
  (bind _loadtornadosound (`self.LoadTornadoSound`))
  (bind (_output_location _output_rotation _output_scale) (`KismetMathLibrary.BreakTransform` (`|GetArrayItem` (`self.StateTornado`))))
  (bind (_output_location_2 _output_rotation_2 _output_scale_2) (`KismetMathLibrary.BreakTransform` (`|GetArrayItem` (`self.StateTornado`) 1)))
  (if (`self.isTornadoCharged?`)
    (if (`self.TornadoOverload`)
      (`/Engine/EditorBlueprintResources/StandardMacros.IsValid` _loadtornadosound
        (:`Is Valid`
          (`AudioComponent.Stop` _loadtornadosound))
        (:`Is Not Valid`
          _))
      (`self.K2_DestroyActor`)
      (else
        (bind _output_get (set `self.State2` (`KismetMathLibrary.MakeTransform` (+ (* _output_location_2 (`self.Forward Vector`)) _player_transform_location_2) _output_rotation_2 _output_scale_2)))))
    (return _output_get)
    (else
      (bind _output_get_2 (set `self.State1` (`KismetMathLibrary.MakeTransform` (+ (* _output_location (`self.Forward Vector`)) _player_transform_location) _output_rotation _output_scale)))
      (return _output_get_2))))

(fn `TimeStateTornado`
  (bind _timekeydown (`self.TimeKeyDown`))
  (if (< _timekeydown 2.0)
    (set `self.isTornadoCharged?` false)
    (return)
    (elif (>= _timekeydown 2.0)
      (if (>= _timekeydown 3.0)
        (set `self.isTornadoCharged?` true)
        (set `self.TornadoOverload` true)
        (return)
        (else
          (set `self.isTornadoCharged?` true)
          (return))))))

(fn `UserConstructionScript`
  (`parent.UserConstructionScript`))