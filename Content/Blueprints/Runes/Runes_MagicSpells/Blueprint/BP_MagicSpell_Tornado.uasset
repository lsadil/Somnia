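; BP_MagicSpell_Tornado is a hold-to-charge tornado spell.
; While pressed, a gated Tick samples and prints key hold time; release classifies it as uncharged, charged or overloaded.
; Overload destroys a charged tornado; otherwise a Timeline lerps the root, with sweep, from the pressed transform to the selected state transform.
; The Etat 1/2 graphs contain only unused MakeTransform nodes that offset StateTornado entries by player location.
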(event `self.ReceiveTick`
  (params (DeltaSeconds :type "Float (single-precision)"))
  (`parent.ReceiveTick` DeltaSeconds)
  (`/Engine/EditorBlueprintResources/StandardMacros.Gate` true :!label _label
    (:`Exit`
      (bind _output_get (set `self.TimeKeyDown` (`PlayerController.GetInputKeyTimeDown` (`GameplayStatics.GetPlayerController` 0) (stale `/Game/Blueprints/Interfaces/BPI_Spell_Magic.Pressed` Key))))
      (`KismetSystemLibrary.PrintString` (`KismetStringLibrary.Conv_DoubleToString` _output_get)))))

(event `/Game/Blueprints/Interfaces/BPI_Spell_Magic.Pressed`
  (params (Transform :type "Transform Structure") (Key :type "Key Structure"))
  (set `self.Player Transform` Transform)
  (goto _label :!via `Open`))

(event `/Game/Blueprints/Interfaces/BPI_Spell_Magic.Released`
  (`KismetSystemLibrary.PrintString` "Released from BP_MS")
  (`|ExecutionSequence`
    (:`then_0`
      (goto _label :!via `Close`))
    (:`then_1`
      (`self.TimeStateTornado`)
      (bind _transform (`self.LaunchTornado`))
      (if (not (`self.TornadoOverload`))
        (bind (_direction _0_1) (`Timeline|Timeline`)
          (:`Update`
            (`SceneComponent.K2_SetWorldTransform` (`self.DefaultSceneRoot`) (`KismetMathLibrary.TLerp` (`self.Player Transform`) _transform _0_1) true false)))))))

(fn `LaunchTornado`
  (returns (Transform :type "Transform Structure"))
  (bind _player_transform_location (`KismetMathLibrary.BreakTransform` (`self.Player Transform`)))
  (bind _player_transform_location_2 (`KismetMathLibrary.BreakTransform` (`self.Player Transform`)))
  (bind (_output_location _output_rotation _output_scale) (`KismetMathLibrary.BreakTransform` (`|GetArrayItem` (`self.StateTornado`))))
  (bind (_output_location_2 _output_rotation_2 _output_scale_2) (`KismetMathLibrary.BreakTransform` (`|GetArrayItem` (`self.StateTornado`) 1)))
  (if (`self.isTornadoCharged?`)
    (if (`self.TornadoOverload`)
      (`self.K2_DestroyActor`)
      (else
        (bind _output_get (set `self.State2` (`KismetMathLibrary.MakeTransform` (+ _output_location_2 _player_transform_location_2) _output_rotation_2 _output_scale_2)))))
    (return _output_get)
    (else
      (bind _output_get_2 (set `self.State1` (`KismetMathLibrary.MakeTransform` (+ _output_location _player_transform_location) _output_rotation _output_scale)))
      (return _output_get_2))))

(fn `TimeStateTornado`
  (bind _timekeydown (`self.TimeKeyDown`))
  (if (< _timekeydown 2.0)
    (set `self.isTornadoCharged?` false)
    (return)
    (elif (>= _timekeydown 2.0)
      (if (>= _timekeydown 3.0)
        (set `self.isTornadoCharged?` true)
        (set `self.TornadoOverload` true)
        (return)
        (else
          (set `self.isTornadoCharged?` true)
          (return))))))

(fn `UserConstructionScript`
  (`parent.UserConstructionScript`))