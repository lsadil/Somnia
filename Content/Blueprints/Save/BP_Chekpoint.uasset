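; BP_Chekpoint is a checkpoint actor that saves the game when BP_Hope enters its box trigger.
; Any overlap plays the audio, then a successful cast to BP_Hope swaps the Paper2D sprite to a golden dreamcatcher and calls Save on BP_Hope.
; After a short delay the sprite switches to the regular dreamcatcher.
; The construction script applies the Sprite variable when it is valid.
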(event `self.Box.OnComponentBeginOverlap`
  (params (OverlappedComponent :type "PrimitiveComponent Object Reference") (OtherActor :type "Actor Object Reference") (OtherComp :type "PrimitiveComponent Object Reference") (OtherBodyIndex :type Integer) (bFromSweep :type Boolean) (SweepResult :type "HitResult Structure (by ref)"))
  (`AudioComponent.Play` (`self.Audio`) 0.0)
  (bind _asbp_hope (cast `/Game/Blueprints/Hope/BP_Hope` OtherActor))
  (`PaperSpriteComponent.SetSprite` (`self.PaperSprite`) "/Game/Assets/UI/HUD/New_Assets/Attrape_rêve_doré_Sprite.Attrape_rêve_doré_Sprite")
  (`/Game/Blueprints/Hope/BP_Hope.Save` _asbp_hope)
  (`KismetSystemLibrary.Delay` 1.5)
  (`PaperSpriteComponent.SetSprite` (`self.PaperSprite`) "/Game/Assets/UI/HUD/New_Assets/Attrape_rêve__Sprite.Attrape_rêve__Sprite"))

(fn `UserConstructionScript`
  (bind _sprite (`self.Sprite`))
  (`/Engine/EditorBlueprintResources/StandardMacros.IsValid` _sprite
    (:`Is Valid`
      (`PaperSpriteComponent.SetSprite` (`self.PaperSprite`) _sprite))))