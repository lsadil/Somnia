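; Game instance for Somnia that owns the save game and persists the player character's progress.
; Init loads BP_SaveGame from a single slot or creates a fresh one, cached as SaveData.
; Save and load functions copy BP_Hope's location, health and staff/tornado flags, and another deletes the slot.
; Destroyed actor IDs are tracked in an in-memory list for lookup, not written to the save.
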(event `self.ReceiveInit`
  (bind _returnvalue (`GameplayStatics.DoesSaveGameExist` (`self.Slot Name`)))
  (if _returnvalue
    (bind _returnvalue_2 (`GameplayStatics.LoadGameFromSlot` (`self.Slot Name`)))
    (bind _asbp_save_game (cast `/Game/Blueprints/Save/BP_SaveGame` _returnvalue_2))
    (set `self.SaveData` _asbp_save_game)
    (else
      (bind _returnvalue_3 (`GameplayStatics.CreateSaveGameObject` "/Game/Blueprints/Save/BP_SaveGame.BP_SaveGame_C"))
      (set `self.SaveData` _returnvalue_3))))

(event `DestroyActor`
  (params (ActorID :type "Name (by ref)"))
  (`KismetArrayLibrary.Array_AddUnique` (`self.DestroyedActor`) ActorID))

(fn `Check If Destroyed`
  (params (ActorID :type "Name (by ref)"))
  (returns (Destroyed :type Boolean))
  (return (> (`KismetArrayLibrary.Array_Find` (`self.DestroyedActor`) ActorID) -1)))

(fn `Delete Data`
  (`GameplayStatics.DeleteGameInSlot` (`self.Slot Name`)))

(fn `Load Data Player`
  (bind (_dataplayer_playerlocation _dataplayer_health _dataplayer_hasstaff_ _dataplayer_hastornado_) (break `/Game/Blueprints/Save/S_DataPlayer` (`/Game/Blueprints/Save/BP_SaveGame.DataPlayer` (`self.SaveData`))))
  (bind _asbp_hope (cast `/Game/Blueprints/Hope/BP_Hope` (`GameplayStatics.GetPlayerCharacter` 0)))
  (`Actor.K2_SetActorLocation` _asbp_hope _dataplayer_playerlocation false false)
  (set `/Game/Blueprints/C_Combat.Health` _dataplayer_health (`/Game/Blueprints/Hope/BP_Hope.Combat` _asbp_hope))
  (set `/Game/Blueprints/Hope/BP_Hope.HasStaff` _dataplayer_hasstaff_ _asbp_hope)
  (set `/Game/Blueprints/Hope/BP_Hope.HasTornado` _dataplayer_hastornado_ _asbp_hope))

(fn `Save Data Player`
  (bind _asbp_hope (cast `/Game/Blueprints/Hope/BP_Hope` (`GameplayStatics.GetPlayerCharacter` 0)))
  (bind _output_get (set `self.As BP Hope` _asbp_hope))
  (set `/Game/Blueprints/Save/BP_SaveGame.DataPlayer` (make `/Game/Blueprints/Save/S_DataPlayer` (`Actor.K2_GetActorLocation` _output_get) (`/Game/Blueprints/C_Combat.Health` (`/Game/Blueprints/Hope/BP_Hope.Combat` _output_get)) (`/Game/Blueprints/Hope/BP_Hope.HasStaff` _output_get) (`/Game/Blueprints/Hope/BP_Hope.HasTornado` _output_get)) (`self.SaveData`))
  (`GameplayStatics.SaveGameToSlot` (`self.SaveData`) (`self.Slot Name`)))