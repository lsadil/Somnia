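; Player controller for Somnia that saves and loads the record of destroyed actors through the game instance and a save slot.
; BeginPlay caches the game instance, which holds the slot name, save object and destroyed-actor data.
; SaveActor reloads the existing slot, overwrites only its destroyed-actor data and writes it back.
; LoadActor copies that data into the game instance, retrying on a short delay until the cached reference is valid.
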(event `self.ReceiveBeginPlay`
  (bind _asgame_instance_somnia (cast `/Game/Blueprints/Save/GameInstance_Somnia` (`GameplayStatics.GetGameInstance`)))
  (set `self.As Game Instance Somnia` _asgame_instance_somnia))

(event `SaveActor`
  (bind _as_game_instance_somnia (`self.As Game Instance Somnia`))
  (bind _savedata (`/Game/Blueprints/Save/GameInstance_Somnia.SaveData` _as_game_instance_somnia))
  ;[1 1 1] Save
  (bind _returnvalue (`GameplayStatics.LoadGameFromSlot` (`/Game/Blueprints/Save/GameInstance_Somnia.Slot Name` _as_game_instance_somnia)))
  (bind _asbp_save_game (cast `/Game/Blueprints/Save/BP_SaveGame` _returnvalue))
  (set `/Game/Blueprints/Save/GameInstance_Somnia.SaveData` _asbp_save_game _as_game_instance_somnia)
  (set `/Game/Blueprints/Save/BP_SaveGame.DestroyedActor` (`/Game/Blueprints/Save/GameInstance_Somnia.DestroyedActor` _as_game_instance_somnia) _savedata)
  (`GameplayStatics.SaveGameToSlot` _savedata (`/Game/Blueprints/Save/GameInstance_Somnia.Slot Name` _as_game_instance_somnia)))

(event `LoadActor`
  (bind _as_game_instance_somnia (`self.As Game Instance Somnia`))
  (bind _as_game_instance_somnia_2 (`self.As Game Instance Somnia`))
  ;[1 1 1] Load
  (`/Engine/EditorBlueprintResources/StandardMacros.IsValid` _as_game_instance_somnia_2 :!label _label
    (:`Is Valid`
      (bind _returnvalue (`GameplayStatics.LoadGameFromSlot` (`/Game/Blueprints/Save/GameInstance_Somnia.Slot Name` _as_game_instance_somnia_2)))
      (bind _asbp_save_game (cast `/Game/Blueprints/Save/BP_SaveGame` _returnvalue))
      (bind _output_get (set `/Game/Blueprints/Save/GameInstance_Somnia.SaveData` _asbp_save_game _as_game_instance_somnia))
      (set `/Game/Blueprints/Save/GameInstance_Somnia.DestroyedActor` (`/Game/Blueprints/Save/BP_SaveGame.DestroyedActor` _output_get) _as_game_instance_somnia))
    (:`Is Not Valid`
      (`KismetSystemLibrary.Delay` 0.2)
      (goto _label))))

(fn `UserConstructionScript`)